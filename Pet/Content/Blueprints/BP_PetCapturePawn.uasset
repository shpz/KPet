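; BP_PetCapturePawn is a pet pawn that shows a computer mesh only while the pet is in the Working state.
; TryActivateComputer and ToggleComputerVisibility share one visibility update driven by CurrentPetState, and OnPetStateChanged re-runs it.
; A two-second BeginPlay timer fires an animation test event (动画测试事件) that forces the Working state and refreshes the computer's visibility.
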(event Custom|动画测试事件
  (Variables|Default|SetCurrentPetState "Working")
  (CallFunction|ToggleComputerVisibility))

(event Custom|TryActivateComputer
  (Rendering|SetVisibility (Variables|Default|GetComputerMesh) (Utilities|Enum|Equal(Enum) (Variables|Default|GetCurrentPetState) "Working") false))

(event Custom|ToggleComputerVisibility
  (Rendering|SetVisibility (Variables|Default|GetComputerMesh) (Utilities|Enum|Equal(Enum) (Variables|Default|GetCurrentPetState) "Working") false))

(event EventBeginPlay
  (Utilities|Time|SetTimerbyEvent (delegate Custom|动画测试事件) 2.0))

(event Collision|EventActorBeginOverlap
  (params (OtherActor :type Actor%20Object%20Reference)))

(event EventTick
  (params (DeltaSeconds :type Float%20%28single-precision%29)))

(event EventOnPetStateChanged
  (params (NewState :type EPetWorkState%20Enum :default "Idle"))
  (CallFunction|TryActivateComputer))

(fn ConstructionScript)